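; Side-scrolling player character with an animated sprite that runs, jumps, climbs ledges and ladders, and fights with a slash combo.
; Velocity sets facing, while tagged overlaps and line traces switch climbing to Flying movement, with a timeline for ledge mantling.
; Slashes lunge forward and pick one of three animations using a Quartz clock as combo timer.
; Overlaps deal damage both ways; taking damage triggers knockback, a material flash and brief invulnerability.
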(event `self.ReceiveTick`
  (params (DeltaSeconds :type "Float (single-precision)"))
  (bind _returnvalue (`self.GetController`))
  (bind _returnvalue_2 (`self.GetController`))
  (if (`self.TurnCharacter`)
    (`parent.ReceiveTick` DeltaSeconds)
    (`/Engine/EditorBlueprintResources/StandardMacros.CompareFloat` (.x (`MovementComponent.Velocity` (`self.GetMovementComponent`)))
      (:`>`
        ;[0 0.4745 1] Look Right
        (`/Engine/EditorBlueprintResources/StandardMacros.IsValid` _returnvalue_2
          (:`Is Valid`
            (`Controller.SetControlRotation` _returnvalue_2 (`KismetMathLibrary.MakeRotator` 0.0)))))
      (:`<`
        ;[0 0.4745 1] Look Left
        (`/Engine/EditorBlueprintResources/StandardMacros.IsValid` _returnvalue
          (:`Is Valid`
            (`Controller.SetControlRotation` _returnvalue (`KismetMathLibrary.MakeRotator` 0.0 0.0 180.0))))))
    (elif (< (`KismetMathLibrary.VSize` (`self.GetVelocity`)) 1.0)
      (set `self.TurnCharacter` true))))

(event `Move`
  (params (ActionValue :type "Vector2D Structure"))
  (bind _returnvalue_x (`KismetMathLibrary.BreakVector` (`self.GetVelocity`)))
  (if (not (or (`self.IsClimbing`) (`self.isLadder`)))
    (`self.AddMovementInput` (1.0 0.0 0.0) ActionValue_X))
  (`self.AddMovementInput` (0.0 0.0 1.0) ActionValue_Y true)
  (if (not (`self.TurnCharacter`))
    (set `self.TurnCharacter` (== ActionValue_X (`KismetMathLibrary.SignOfFloat` _returnvalue_x)))))

(event `self.ReceiveBeginPlay`
  (bind _returnvalue (`QuartzSubsystem.CreateNewClock` :`self` (subsystem `QuartzSubsystem`) :`ClockName` "Quartz Timer"))
  (bind _output_get (set `self.Quartz Clock` _returnvalue))
  (`QuartzClockHandle.StartClock` _output_get)
  (bind _returnvalue_2 (`PrimitiveComponent.CreateDynamicMaterialInstance` (`self.Sprite`) 0 null "None"))
  (set `self.Dynamic Sprite Mat` _returnvalue_2))

(event `self.OnJumped`
  (`PaperZDAnimInstance.JumpToNode` (`PaperZDAnimationComponent.AnimInstance` (`self.AnimationComponent`)) "Airborne" "None" :!label _label))

(event `self.OnWalkingOffLedge`
  (params (PreviousFloorImpactNormal :type "Vector Structure (by ref)") (PreviousFloorContactNormal :type "Vector Structure (by ref)") (PreviousLocation :type "Vector Structure (by ref)") (TimeDelta :type "Float (single-precision)"))
  (goto _label))

(event `self.OnLanded`
  (params (Hit :type "HitResult Structure (by ref)"))
  (bind _returnvalue_x (`KismetMathLibrary.BreakVector2D` (`|GetInputActionValue`)))
  (if (== _returnvalue_x 0.0)
    (`PaperZDAnimInstance.JumpToNode` (`PaperZDAnimationComponent.AnimInstance` (`self.AnimationComponent`)) "Landed" "None")))

(event `Slash`
  (bind _quartz_clock (`self.Quartz Clock`))
  (bind _returnvalue (`QuartzClockHandle.IsClockRunning` _quartz_clock))
  (if _returnvalue
    (`MovementComponent.StopMovementImmediately` (`self.CharacterMovement`))
    (`Controller.SetIgnoreMoveInput` (`GameplayStatics.GetPlayerController` 0) true)
    (set `MovementComponent.Velocity` (* (`self.GetActorForwardVector`) 500.0) (`self.CharacterMovement`))
    (set `PrimitiveComponent.bGenerateOverlapEvents` true (`self.ComboCollision`))
    (`self.ComboSlash` _quartz_clock)))

(event `CheckLedge`
  (bind _returnvalue (`self.K2_GetActorLocation`))
  (bind (_returnvalue_x _returnvalue_y) (`KismetMathLibrary.BreakVector2D` (`|GetInputActionValue`)))
  (bind (_locorig_x _locorig_y _locorig_z) (`KismetMathLibrary.BreakVector` (`self.LocOrig`)))
  (bind (_returnvalue_x_2 _returnvalue_y_2 _returnvalue_z) (`KismetMathLibrary.BreakVector` (+ (`self.LocOrig`) (+ (* (`self.GetActorForwardVector`) 100.0) (* (`KismetMathLibrary.GetUpVector` (struct)) 100.0)))))
  (bind (_outhit _returnvalue_2) (`KismetSystemLibrary.LineTraceSingle` :`Start` _returnvalue :`End` (+ _returnvalue (* (`self.GetActorForwardVector`) 100.0)) :`TraceChannel` "TraceTypeQuery1" :`DrawDebugType` "ForDuration"))
  (if (not _returnvalue_2)
    (`self.SetIsClimbing` false)
    (if (> _returnvalue_y 0.0)
      (`Controller.SetIgnoreMoveInput` (`GameplayStatics.GetPlayerController` 0) true)
      (set `self.LocOrig` (`self.K2_GetActorLocation`))
      (bind (_direction _alphay _alphax) (`Timeline|MoveToPoint` :!via `PlayFromStart`)
        (:`Update`
          (`self.K2_SetActorLocation` (`KismetMathLibrary.MakeVector` (`KismetMathLibrary.Lerp` _locorig_x _returnvalue_x_2 _alphax) _locorig_y (`KismetMathLibrary.Lerp` _locorig_z _returnvalue_z _alphay))))
        (:`Finished`
          (`Controller.SetIgnoreMoveInput` (`GameplayStatics.GetPlayerController` 0) false))))))

(event `self.Hitbox.OnComponentBeginOverlap`
  (params (OverlappedComponent :type "PrimitiveComponent Object Reference") (OtherActor :type "Actor Object Reference") (OtherComp :type "PrimitiveComponent Object Reference") (OtherBodyIndex :type Integer) (bFromSweep :type Boolean) (SweepResult :type "HitResult Structure (by ref)"))
  (if (and (`self.bCanBeDamaged`) (`self.ActorHasTag` OtherActor "enemy"))
    (`GameplayStatics.ApplyDamage` self 50.0 null OtherActor)
    (set `self.bCanBeDamaged` false)
    (`Controller.SetIgnoreMoveInput` (`GameplayStatics.GetPlayerController` 0) true)))

(event `self.ReceiveAnyDamage`
  (params (Damage :type "Float (single-precision)") (DamageType :type "DamageType Object Reference") (InstigatedBy :type "Controller Object Reference") (DamageCauser :type "Actor Object Reference"))
  (`self.SetIsClimbing` false)
  (`self.SetIsLadder` false)
  (`PaperZDAnimInstance.JumpToNode` (`PaperZDAnimationComponent.AnimInstance` (`self.AnimationComponent`)) "Damage" "None")
  (set `MovementComponent.Velocity` (* (`self.GetActorForwardVector` DamageCauser) 1000.0) (`self.CharacterMovement`))
  (bind (_direction _alpha) (`Timeline|Timeline` :!via `PlayFromStart`)
    (:`Update`
      (`MaterialInstanceDynamic.SetScalarParameterValue` (`self.Dynamic Sprite Mat`) "FlashMultiplier" _alpha))
    (:`Finished`
      (set `self.bCanBeDamaged` true)
      (`Controller.SetIgnoreMoveInput` (`GameplayStatics.GetPlayerController` 0) false))))

(event `self.ComboCollision.OnComponentBeginOverlap`
  (params (OverlappedComponent :type "PrimitiveComponent Object Reference") (OtherActor :type "Actor Object Reference") (OtherComp :type "PrimitiveComponent Object Reference") (OtherBodyIndex :type Integer) (bFromSweep :type Boolean) (SweepResult :type "HitResult Structure (by ref)"))
  (for _array_element (`Actor.Tags` OtherActor)
    (switch `name` _array_element
      (:`hitable`
        (set `MovementComponent.Velocity` (* (* (`self.GetActorForwardVector`) -1.0) 500.0) (`self.CharacterMovement`))
        (set `self.TurnCharacter` false))
      (:`enemy`
        (`GameplayStatics.ApplyDamage` OtherActor 50.0 null self)
        (set `Actor.bCanBeDamaged` false OtherActor)))))

(event `self.Ledge Detector.OnComponentBeginOverlap`
  (params (OverlappedComponent :type "PrimitiveComponent Object Reference") (OtherActor :type "Actor Object Reference") (OtherComp :type "PrimitiveComponent Object Reference") (OtherBodyIndex :type Integer) (bFromSweep :type Boolean) (SweepResult :type "HitResult Structure (by ref)"))
  (bind _returnvalue (`self.K2_GetActorLocation`))
  (if (`ActorComponent.ComponentHasTag` OtherComp "climb")
    (`self.SetIsClimbing` true)
    (bind (_outhit _returnvalue_2) (`KismetSystemLibrary.LineTraceSingle` _returnvalue (+ _returnvalue (* (`self.GetActorForwardVector`) 100.0)) "TraceTypeQuery1"))
    (if _returnvalue_2
      (`MovementComponent.StopMovementImmediately` (`self.CharacterMovement`))
      (`self.K2_SetActorLocation` (+ (`.Location` (`GameplayStatics.BreakHitResult` _outhit)) (* (`self.GetActorForwardVector`) -50.0)) false true)
      (`PaperZDAnimInstance.JumpToNode` (`PaperZDAnimationComponent.AnimInstance` (`self.AnimationComponent`)) "ClimbingSide" "None"))))

(event `LadderDetect`
  (bind _ladder_detector (`self.Ladder Detector`))
  (bind _outcomponents (`KismetSystemLibrary.ComponentOverlapComponents` _ladder_detector (`SceneComponent.K2_GetComponentToWorld` _ladder_detector) (`|MakeArray` "ObjectTypeQuery1" "ObjectTypeQuery2" "ObjectTypeQuery3" :!type "EObjectTypeQuery Enum") "/Script/Engine.BoxComponent" (`|MakeArray` self :!type "Actor Object Reference")))
  (for _array_element _outcomponents
    (if (`ActorComponent.ComponentHasTag` _array_element "ladder")
      (`self.SetIsLadder` true)
      (`PaperZDAnimInstance.JumpToNode` (`PaperZDAnimationComponent.AnimInstance` (`self.AnimationComponent`)) "Climbing" "None"))))

(event `self.Ladder Detector.OnComponentEndOverlap`
  (params (OverlappedComponent :type "PrimitiveComponent Object Reference") (OtherActor :type "Actor Object Reference") (OtherComp :type "PrimitiveComponent Object Reference") (OtherBodyIndex :type Integer))
  (`self.SetIsLadder` false))

(fn `ComboSlash`
  (params (InputPin :type "QuartzClockHandle Object Reference"))
  (bind _animinstance (`PaperZDAnimationComponent.AnimInstance` (`self.AnimationComponent`)))
  (switch `int` (`self.Combo`)
    (:`0`
      (`QuartzClockHandle.StopClock` InputPin false)
      (`PaperZDAnimInstance.JumpToNode` _animinstance "Slash1" "None")
      (`/Engine/EditorBlueprintResources/StandardMacros.IncrementInt` (`self.Combo`)))
    (:`1`
      (bind _returnvalue (`QuartzClockHandle.GetEstimatedRunTime` InputPin))
      (`QuartzClockHandle.StopClock` InputPin false)
      (if (<= _returnvalue (`self.MaxComboTime`))
        (`PaperZDAnimInstance.JumpToNode` _animinstance "Slash2" "None")
        (`/Engine/EditorBlueprintResources/StandardMacros.IncrementInt` (`self.Combo`))
        (else
          (`PaperZDAnimInstance.JumpToNode` _animinstance "Slash1" "None"))))
    (:`2`
      (bind _returnvalue_2 (`QuartzClockHandle.GetEstimatedRunTime` InputPin))
      (`QuartzClockHandle.StopClock` InputPin false)
      (if (<= _returnvalue_2 (`self.MaxComboTime`))
        (`PaperZDAnimInstance.JumpToNode` _animinstance "Slash3" "None")
        (else
          (`PaperZDAnimInstance.JumpToNode` _animinstance "Slash1" "None")))
      (set `self.Combo` 0))))

(fn `SetIsClimbing`
  (params (value :type Boolean))
  (bind _charactermovement (`self.CharacterMovement`))
  (set `self.IsClimbing` value)
  (if value
    (`CharacterMovementComponent.SetMovementMode` _charactermovement "MOVE_Flying" 0)
    (else
      (`CharacterMovementComponent.SetMovementMode` _charactermovement "MOVE_Walking" 0))))

(fn `SetIsLadder`
  (params (value :type Boolean))
  (bind _charactermovement (`self.CharacterMovement`))
  (set `self.isLadder` value)
  (if value
    (`CharacterMovementComponent.SetMovementMode` _charactermovement "MOVE_Flying" 0)
    (else
      (`CharacterMovementComponent.SetMovementMode` _charactermovement "MOVE_Walking" 0))))

(fn `SpawnDust`
  (bind (_returnvalue_location _returnvalue_rotation) (`KismetMathLibrary.BreakTransform` (`SceneComponent.K2_GetComponentToWorld` (`self.Sprite`))))
  (`|SpawnActorFromClass` "/Game/Blueprints/BP_LandDust.BP_LandDust_C" (`KismetMathLibrary.MakeTransform` _returnvalue_location _returnvalue_rotation) "Undefined" "MultiplyWithRoot" null null))

(fn `UserConstructionScript`)