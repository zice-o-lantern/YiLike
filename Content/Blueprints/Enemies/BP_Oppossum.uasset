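; BP_Oppossum is a patrolling enemy character that constantly walks along its forward vector.
; WallDetector begin-overlap and LedgeDetector end-overlap events call TurnChar to turn it at walls and ledges.
; Damage lowers HP, knocks it along the damage causer's forward vector, and plays a timeline that flashes the sprite through a dynamic material parameter, setting CanBeDamaged true on each update.
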(event `self.ReceiveTick`
  (params (DeltaSeconds :type "Float (single-precision)"))
  (`parent.ReceiveTick` DeltaSeconds)
  (`self.AddMovementInput` (`self.GetActorForwardVector`)))

(event `self.Wall Detector.OnComponentBeginOverlap`
  (params (OverlappedComponent :type "PrimitiveComponent Object Reference") (OtherActor :type "Actor Object Reference") (OtherComp :type "PrimitiveComponent Object Reference") (OtherBodyIndex :type Integer) (bFromSweep :type Boolean) (SweepResult :type "HitResult Structure (by ref)"))
  (`self.TurnChar`))

(event `self.Ledge Detector.OnComponentEndOverlap`
  (params (OverlappedComponent :type "PrimitiveComponent Object Reference") (OtherActor :type "Actor Object Reference") (OtherComp :type "PrimitiveComponent Object Reference") (OtherBodyIndex :type Integer))
  (`self.TurnChar`))

(event `self.ReceiveAnyDamage`
  (params (Damage :type "Float (single-precision)") (DamageType :type "DamageType Object Reference") (InstigatedBy :type "Controller Object Reference") (DamageCauser :type "Actor Object Reference"))
  (`self.SetHP` (- (`self.HP`) Damage))
  (set `MovementComponent.Velocity` (* (`self.GetActorForwardVector` DamageCauser) 3000.0) (`self.CharacterMovement`))
  (bind (_direction _alpha) (`Timeline|FlashTimeline` :!via `PlayFromStart`)
    (:`Update`
      (`MaterialInstanceDynamic.SetScalarParameterValue` (`self.Dynamic Sprite Mat`) "FlashMultiplier" _alpha)
      (set `self.bCanBeDamaged` true))))

(fn `UserConstructionScript`
  (`parent.UserConstructionScript`))