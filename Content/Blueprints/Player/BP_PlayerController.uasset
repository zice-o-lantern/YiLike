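; Player controller that adds the IMC_Player Enhanced Input context and forwards move, jump, slash and dash input to the possessed BP_Player.
; Jumping while holding down deactivates collision on overlapped "through"-tagged BP_Through actors instead of jumping.
; Otherwise, jumping from a climb or ladder clears climbing and pushes the pawn backward.
; Movement input also triggers ledge checks while climbing and ladder detection when pressing up off a ladder.
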(event `self.ReceiveBeginPlay`
  (bind _returnvalue (pcsubsystem `EnhancedInputLocalPlayerSubsystem` self))
  (`/Engine/EditorBlueprintResources/StandardMacros.IsValid` _returnvalue
    (:`Is Valid`
      (`EnhancedInputSubsystemInterface.AddMappingContext` _returnvalue "/Game/IA/IMC_Player.IMC_Player" 0 (struct)))))

(event `self.ReceivePossess`
  (params (PossessedPawn :type "Pawn Object Reference"))
  (bind _asbp_player (cast `/Game/Blueprints/Player/BP_Player` PossessedPawn))
  (set `self.PlayerPawn` _asbp_player))

(event `EnhancedInput|/Game/IA/IA_Jump`
  (params (ActionValue :type Boolean) (ElapsedSeconds :type "Float (double-precision)") (TriggeredSeconds :type "Float (double-precision)") (InputAction :type "InputAction Object Reference" :default "/Game/IA/IA_Jump.IA_Jump"))
  (bind (_returnvalue_x _returnvalue_y) (`KismetMathLibrary.BreakVector2D` (`|GetInputActionValue`)))
  (bind _playerpawn (`self.PlayerPawn`))
  (bind _playerpawn_2 (`self.PlayerPawn`))
  (bind _capsulecomponent (`Character.CapsuleComponent` (`self.PlayerPawn`)))
  (:`Started`
    (if (< _returnvalue_y 0.0)
      (bind _outcomponents (`KismetSystemLibrary.ComponentOverlapComponents` _capsulecomponent (`SceneComponent.K2_GetComponentToWorld` _capsulecomponent) (`|MakeArray` "ObjectTypeQuery1" "ObjectTypeQuery3" "ObjectTypeQuery2" :!type "EObjectTypeQuery Enum")))
      (for _array_element _outcomponents
        (if (`ActorComponent.ComponentHasTag` _array_element "through")
          (bind _asbp_through (cast `/Game/Blueprints/BP_Through` (`ActorComponent.GetOwner` _array_element)))
          (`/Game/Blueprints/BP_Through.DeactivateCollision` _asbp_through (`self.PlayerPawn`))))
      (else
        (if (or (`/Game/Blueprints/Player/BP_Player.IsClimbing` _playerpawn_2) (`/Game/Blueprints/Player/BP_Player.isLadder` _playerpawn_2))
          (`/Game/Blueprints/Player/BP_Player.SetIsClimbing` _playerpawn_2 false)
          (set `MovementComponent.Velocity` (* (* (`self.GetActorForwardVector` _playerpawn_2) -1.0) 300.0) (`Character.CharacterMovement` _playerpawn_2)))
        (`Character.Jump` _playerpawn))))
  (:`Completed`
    (`Character.StopJumping` _playerpawn)))

(event `EnhancedInput|/Game/IA/IA_Move`
  (params (ActionValue :type "Vector2D Structure") (ElapsedSeconds :type "Float (double-precision)") (TriggeredSeconds :type "Float (double-precision)") (InputAction :type "InputAction Object Reference" :default "/Game/IA/IA_Move.IA_Move"))
  (bind _playerpawn (`self.PlayerPawn`))
  (:`Triggered`
    (`/Game/Blueprints/Player/BP_Player.Move` _playerpawn ActionValue)
    (if (`/Game/Blueprints/Player/BP_Player.IsClimbing` _playerpawn)
      (`/Game/Blueprints/Player/BP_Player.CheckLedge` _playerpawn))
    (if (and (> (`.Y` (`KismetMathLibrary.BreakVector2D` ActionValue)) 0.0) (not (`/Game/Blueprints/Player/BP_Player.isLadder` _playerpawn)))
      (`/Game/Blueprints/Player/BP_Player.LadderDetect` _playerpawn))))

(event `EnhancedInput|/Game/IA/IA_Action`
  (params (ActionValue :type Boolean) (ElapsedSeconds :type "Float (double-precision)") (TriggeredSeconds :type "Float (double-precision)") (InputAction :type "InputAction Object Reference" :default "/Game/IA/IA_Action.IA_Action"))
  (:`Started`
    (`/Game/Blueprints/Player/BP_Player.Slash` (`self.PlayerPawn`))))

(event `EnhancedInput|/Game/IA/IA_Dash`
  (params (ActionValue :type Boolean) (ElapsedSeconds :type "Float (double-precision)") (TriggeredSeconds :type "Float (double-precision)") (InputAction :type "InputAction Object Reference" :default "/Game/IA/IA_Dash.IA_Dash"))
  (:`Triggered`
    (`/Game/Blueprints/Player/BP_Player.Dash` (`self.PlayerPawn`))))

(fn `UserConstructionScript`)