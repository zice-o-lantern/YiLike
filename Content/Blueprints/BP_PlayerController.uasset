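; Player controller that turns Enhanced Input actions into commands on the possessed BP_Player pawn.
; BeginPlay adds the IMC_Player mapping context, and Possess casts and caches the pawn as PlayerPawn.
; Jump, move and action inputs are forwarded to that pawn's Jump/StopJumping, Move and Slash functions, so the controller holds no movement or attack logic itself.
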(event `self.ReceiveBeginPlay`
  (bind _returnvalue (pcsubsystem `EnhancedInputLocalPlayerSubsystem` self))
  (`/Engine/EditorBlueprintResources/StandardMacros.IsValid` _returnvalue
    (:`Is Valid`
      (`EnhancedInputSubsystemInterface.AddMappingContext` _returnvalue "/Game/IA/IMC_Player.IMC_Player" 0 (struct)))))

(event `self.ReceivePossess`
  (params (PossessedPawn :type "Pawn Object Reference"))
  (bind _asbp_player (cast `/Game/Blueprints/BP_Player` PossessedPawn))
  (set `self.PlayerPawn` _asbp_player))

(event `EnhancedInput|/Game/IA/IA_Jump`
  (params (ActionValue :type Boolean) (ElapsedSeconds :type "Float (double-precision)") (TriggeredSeconds :type "Float (double-precision)") (InputAction :type "InputAction Object Reference" :default "/Game/IA/IA_Jump.IA_Jump"))
  (bind _playerpawn (`self.PlayerPawn`))
  (:`Started`
    (`Character.Jump` _playerpawn))
  (:`Completed`
    (`Character.StopJumping` _playerpawn)))

(event `EnhancedInput|/Game/IA/IA_Move`
  (params (ActionValue :type "Float (double-precision)") (ElapsedSeconds :type "Float (double-precision)") (TriggeredSeconds :type "Float (double-precision)") (InputAction :type "InputAction Object Reference" :default "/Game/IA/IA_Move.IA_Move"))
  (:`Triggered`
    (`/Game/Blueprints/BP_Player.Move` (`self.PlayerPawn`) ActionValue)))

(event `EnhancedInput|/Game/IA/IA_Action`
  (params (ActionValue :type Boolean) (ElapsedSeconds :type "Float (double-precision)") (TriggeredSeconds :type "Float (double-precision)") (InputAction :type "InputAction Object Reference" :default "/Game/IA/IA_Action.IA_Action"))
  (:`Started`
    (`/Game/Blueprints/BP_Player.Slash` (`self.PlayerPawn`))))

(fn `UserConstructionScript`)