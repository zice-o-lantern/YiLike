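; BP_Through is a one-way platform that BP_Player can jump up through and drop down through.
; A Detector overlap switches the Collision component's Pawn response to Block, immediately for a descending player, otherwise after a short delay with a "Through" animation jump.
; Leaving the Detector restores Ignore.
; A DeactivateCollision event also sets Ignore and jumps the player's animation to "FallThrough".
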(event `self.Detector.OnComponentBeginOverlap`
  (params (OverlappedComponent :type "PrimitiveComponent Object Reference") (OtherActor :type "Actor Object Reference") (OtherComp :type "PrimitiveComponent Object Reference") (OtherBodyIndex :type Integer) (bFromSweep :type Boolean) (SweepResult :type "HitResult Structure (by ref)"))
  (bind _asbp_player (cast `/Game/Blueprints/Player/BP_Player` OtherActor))
  (bind (_velocity_x _velocity_y _velocity_z) (`KismetMathLibrary.BreakVector` (`MovementComponent.Velocity` (`Character.CharacterMovement` _asbp_player))))
  (if (< _velocity_z 0.0)
    (`PrimitiveComponent.SetCollisionResponseToChannel` (`self.Collision`) "ECC_Pawn" "ECR_Block")
    (else
      (`KismetSystemLibrary.Delay` 0.2)
      (`PrimitiveComponent.SetCollisionResponseToChannel` (`self.Collision`) "ECC_Pawn" "ECR_Block")
      (`PaperZDAnimInstance.JumpToNode` (`PaperZDAnimationComponent.AnimInstance` (`PaperZDCharacter.AnimationComponent` _asbp_player)) "Through" "None"))))

(event `self.Detector.OnComponentEndOverlap`
  (params (OverlappedComponent :type "PrimitiveComponent Object Reference") (OtherActor :type "Actor Object Reference") (OtherComp :type "PrimitiveComponent Object Reference") (OtherBodyIndex :type Integer))
  (bind _asbp_player (cast `/Game/Blueprints/Player/BP_Player` OtherActor))
  (`PrimitiveComponent.SetCollisionResponseToChannel` (`self.Collision`) "ECC_Pawn" "ECR_Ignore"))

(event `DeactivateCollision`
  (params (Character :type "Character Object Reference"))
  (bind _asbp_player (cast `/Game/Blueprints/Player/BP_Player` Character))
  (`PrimitiveComponent.SetCollisionResponseToChannel` (`self.Collision`) "ECC_Pawn" "ECR_Ignore")
  (`PaperZDAnimInstance.JumpToNode` (`PaperZDAnimationComponent.AnimInstance` (`PaperZDCharacter.AnimationComponent` _asbp_player)) "FallThrough" "None"))

(fn `UserConstructionScript`)