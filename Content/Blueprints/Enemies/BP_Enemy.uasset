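; BP_Enemy is a sprite-based enemy actor with hit points, a turn-around action and death.
; On BeginPlay it creates and stores a dynamic material instance for its sprite, while Tick only calls the parent.
; TurnChar flips the actor by combining its rotation with a 180-degree turn.
; SetHP stores the new value and, at zero or below, schedules Death for the next tick, which destroys the actor.
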(event `self.ReceiveBeginPlay`
  (bind _returnvalue (`PrimitiveComponent.CreateDynamicMaterialInstance` (`self.Sprite`) 0 null "None"))
  (set `self.Dynamic Sprite Mat` _returnvalue))

(event `self.ReceiveTick`
  (params (DeltaSeconds :type "Float (single-precision)"))
  (`parent.ReceiveTick` 0.0))

(fn `Death`
  (`self.K2_DestroyActor`))

(fn `SetHP`
  (params (Value :type "Float (double-precision)"))
  (bind _output_get (set `self.HP` Value))
  (if (<= _output_get 0.0)
    (`KismetSystemLibrary.K2_SetTimerForNextTick` null "Death")))

(fn `TurnChar`
  (`self.K2_SetActorRotation` (`KismetMathLibrary.ComposeRotators` (`self.K2_GetActorRotation`) (struct :`Yaw` 180.0))))

(fn `UserConstructionScript`)